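; BP_Item_AxeHandle_Single is an axe handle item Blueprint in the Overview scene content of the point-and-click toolkit.
; It exposes interaction and inventory functions, but all return defaults: use and item receipt fail, it is not an inventory item, and its name is "None".
; The construction script only calls its parent, and the event graph holds only disabled placeholder events, so this Blueprint adds no behavior of its own.
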(fn `GetItemName`
  (returns (NewParam :type Name))
  (return "None"))

(fn `IsInventoryItem`
  (returns (return :type Boolean))
  (return false))

(fn `RecieveItem`
  (params (ItemName :type Name))
  (returns (Valid :type Boolean) (Consumed :type Boolean))
  (return false false))

(fn `UseObject`
  (params (InteractingCharacter :type "/Game/PNCTookit/Blueprints/Characters/BP_PNCCharacter_Parent Object Reference"))
  (returns (Success :type Boolean))
  (return false))

(fn `UserConstructionScript`
  (`parent.UserConstructionScript`))