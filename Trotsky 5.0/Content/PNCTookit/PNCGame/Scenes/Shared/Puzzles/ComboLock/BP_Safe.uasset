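; Interactable safe for the point-and-click toolkit that opens its door when the player solves its combination lock puzzle.
; Using it starts the puzzle with itself as owner and a hard-coded code.
; A successful result deactivates the safe, marks it used and plays a timeline that yaws the door mesh open.
; On BeginPlay, an already used safe plays the same timeline to restore its open state.
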(event `self.ReceiveBeginPlay`
  (`parent.ReceiveBeginPlay`)
  (if (`self.bIsUsed`)
    (bind (_direction _float) (`Timeline|OpenDoor` :!label _label)
      (:`Update`
        (`SceneComponent.K2_SetRelativeRotation` (`self.SafeDoorMesh`) (`KismetMathLibrary.MakeRotator` 0.0 0.0 _float) false false)))))

(event `OpenSafeDoor`
  (set `self.bIsUsed` true)
  (goto _label :!via `PlayFromStart`))

(fn `ReturnPuzzleResult`
  (params (Success :type Boolean))
  (returns (Return :type Boolean))
  (if Success
    (set `self.bIsActive` false)
    (`self.OpenSafeDoor`))
  (return true))

(fn `UseObject`
  (params (InteractingCharacter :type "/Game/PNCTookit/Blueprints/Characters/BP_PNCCharacter_Parent Object Reference"))
  (returns (Success :type Boolean))
  (`/Game/PNCTookit/Blueprints/Gameplay/Puzzles/BPFL_PuzzleHelpers.StartPuzzle` "NewEnumerator4" self 1947)
  (return true))

(fn `UserConstructionScript`
  (`parent.UserConstructionScript`))