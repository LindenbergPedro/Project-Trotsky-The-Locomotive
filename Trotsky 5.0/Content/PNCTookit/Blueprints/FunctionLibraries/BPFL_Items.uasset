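; Blueprint function library of item helpers for a point-and-click toolkit, covering inventory lookup, item data and item combining.
; Inventory queries read the player controller's InventoryComponent.
; Item data comes from searching the scene manager's active item DataTables by row name, with debug prints when nothing is found.
; The combine check tests each item's CanCombineWith list in both orders and returns the created item and its dialogue.
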(fn `CanItemsBeCombined`
  (params (Item1 :type Name) (Item2 :type Name))
  (returns (Valid :type Boolean) (Item_Created :type Name) (OnCombinedDialogue :type Name))
  (locals (CheckItem1 :type Name :default "None") (CheckItem2 :type Name :default "None") (bIsFlipped :type Boolean))
  ;[0.4662 1 0.9502 0.3] Returns whether or not the given two items can be combined. If valid, the function also returns the combined item name
  ;
  ; Update 1.1 - Added return
  (set `local.CheckItem1` Item1)
  (set `local.CheckItem2` (`local.Item2`))
  (bind (_returnvalid _itemdata) (`self.GetItemData` (`local.CheckItem1`) :!label _label))
  (if _returnvalid
    (for _array_element (`.CanCombineWith_33_C9AAE7754AE7B65E6552F5B688E447E6` (break `/Game/PNCTookit/Blueprints/Gameplay/Items/SItemList` _itemdata))
      (bind (_otheritem _itemcreated _oncombineddialogue) (break `/Game/PNCTookit/Blueprints/Gameplay/Items/SCombinedItems` _array_element))
      (if (== _otheritem (`local.CheckItem2`))
        (return true _itemcreated _oncombineddialogue)))
    (if (`local.bIsFlipped`)
      _
      (else
        (set `local.bIsFlipped` true)
        (set `local.CheckItem1` (`local.Item2`))
        (set `local.CheckItem2` (`local.Item1`))
        (goto _label)))
    (else
      (`/Game/PNCTookit/Blueprints/FunctionLibraries/BPFL_DeveloperHelpers.Custom Print` (`KismetStringLibrary.Concat_StrStr` "\"" (`KismetStringLibrary.Conv_NameToString` (`local.Item1`)) "\" cannot be combined with \"" (`KismetStringLibrary.Conv_NameToString` (`local.Item2`))) "NewEnumerator0" true)))
  (return false "None" "None"))

(fn `FindItemInInventory`
  (params (Item :type Name))
  (returns (return :type "/Game/PNCTookit/Blueprints/Gameplay/Items/SInventoryItem Structure") (bFound :type Boolean))
  ;[0.4662 1 0.9502 0.3] Return a given items data structure from the players inventory
  (bind _asbp_pncplayer_controller (cast `/Game/PNCTookit/Blueprints/BP_PNCPlayerController` (`GameplayStatics.GetPlayerController` null))
    (:`then`
      (return (`BlueprintMapLibrary.Map_Find` (`/Game/PNCTookit/Blueprints/Components/BP_InventoryComponent.Get Inventory` (`/Game/PNCTookit/Blueprints/BP_PNCPlayerController.InventoryComponent` _asbp_pncplayer_controller)) Item) true))
    (:`CastFailed`
      (return (struct) false))))

(fn `GetItemData`
  (params (ItemName :type Name))
  (returns (ReturnValid :type Boolean) (ItemData :type "/Game/PNCTookit/Blueprints/Gameplay/Items/SItemList Structure"))
  ;[0.4662 1 0.9502 0.3] Returns the given items data structure
  (for _array_element (`/Game/PNCTookit/Blueprints/BP_SceneManagerBase.ActiveItemsDataTables` (`/Game/PNCTookit/Blueprints/FunctionLibraries/BPFL_GameFramework.Get Scene Manager` null))
    (bind _outrownames (`DataTableFunctionLibrary.GetDataTableRowNames` _array_element))
    (if (`KismetArrayLibrary.Array_Contains` _outrownames ItemName)
      (bind _returnvalue (`|GetDataTableRow` _array_element ItemName)
        (:`then`
          (return true _returnvalue))
        (:`RowNotFound`
          (return false)))))
  (`/Game/PNCTookit/Blueprints/FunctionLibraries/BPFL_DeveloperHelpers.Custom Print` (`KismetStringLibrary.Concat_StrStr` "\"" (`KismetStringLibrary.Conv_NameToString` ItemName) "\" Item Row Name could not be found.") "NewEnumerator0" true)
  (`/Game/PNCTookit/Blueprints/FunctionLibraries/BPFL_DeveloperHelpers.Custom Print` "Tip: Maybe your item has not been added \nto your active list(?). lD not be found." "NewEnumerator0" true)
  (return false))

(fn `GetPlayerInventory`
  (returns (Inventory :type "Map of Name to /Game/PNCTookit/Blueprints/Gameplay/Items/SInventoryItem Structure"))
  (bind _controller (`/Game/PNCTookit/Blueprints/FunctionLibraries/BPFL_Controller.GetPNC_PlayerController` null))
  ;[1 0.4423 0.1995 0.3] Return a list ofitems found in the players inventory
  (`/Engine/EditorBlueprintResources/StandardMacros.IsValid` _controller
    (:`Is Valid`
      (return (`/Game/PNCTookit/Blueprints/Components/BP_InventoryComponent.Get Inventory` (`/Game/PNCTookit/Blueprints/BP_PNCPlayerController.InventoryComponent` _controller))))
    (:`Is Not Valid`
      (return))))