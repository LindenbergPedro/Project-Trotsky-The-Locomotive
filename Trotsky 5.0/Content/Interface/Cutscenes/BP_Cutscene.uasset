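; BP_Cutscene is a timed cutscene actor that plays shortly after BeginPlay and again whenever its Box component registers an overlap, with no filter.
; StartCutscene disables player input, switches the view target to a referenced camera and shows the WB_Cutscene01 widget.
; After a fixed delay, EndCutscene removes the widget, returns the view to the PNC camera manager and restores input.
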(event `self.ReceiveBeginPlay`
  (`KismetSystemLibrary.Delay` 0.2)
  (`self.StartCutscene`)
  (`KismetSystemLibrary.Delay` 3.0)
  (`self.EndCutscene`))

(event `self.Box.OnComponentBeginOverlap`
  (params (OverlappedComponent :type "PrimitiveComponent Object Reference") (OtherActor :type "Actor Object Reference") (OtherComp :type "PrimitiveComponent Object Reference") (OtherBodyIndex :type Integer) (bFromSweep :type Boolean) (SweepResult :type "HitResult Structure (by ref)"))
  (`self.StartCutscene`)
  (`KismetSystemLibrary.Delay` 3.0)
  (`self.EndCutscene`))

(fn `EndCutscene`
  (`Widget.RemoveFromParent` (`self.WB_CutsceneRefer`))
  (`PlayerController.SetViewTargetWithBlend` (`/Game/PNCTookit/Blueprints/FunctionLibraries/BPFL_Controller.GetPNC_PlayerController`) (`/Game/PNCTookit/Blueprints/FunctionLibraries/BPFL_Controller.GetPNC_CameraManager`) 0.0 "VTBlend_Linear" 0.0 false)
  (`/Game/PNCTookit/Blueprints/BP_PNCPlayerController.SetInputEnabled` (`/Game/PNCTookit/Blueprints/FunctionLibraries/BPFL_Controller.GetPNC_PlayerController`) true))

(fn `StartCutscene`
  (`/Game/PNCTookit/Blueprints/BP_PNCPlayerController.SetInputEnabled` (`/Game/PNCTookit/Blueprints/FunctionLibraries/BPFL_Controller.GetPNC_PlayerController`) false)
  (`PlayerController.SetViewTargetWithBlend` (`/Game/PNCTookit/Blueprints/FunctionLibraries/BPFL_Controller.GetPNC_PlayerController`) (`self.CameraRefer`) 0.0 "VTBlend_Linear" 0.0 false)
  (bind _returnvalue (`|CreateWidget` "/Game/Interface/Cutscenes/WB_Cutscene01.WB_Cutscene01_C"))
  (bind _output_get (set `self.WB_CutsceneRefer` _returnvalue))
  (`UserWidget.AddToViewport` _output_get 0))

(fn `UserConstructionScript`)