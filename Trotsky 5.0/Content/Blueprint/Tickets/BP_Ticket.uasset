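; BP_Ticket is an interactable ticket actor that shows its Message in an on-screen WBP_Ticket widget when used.
; BeginPlay creates and caches the ticket widget and a WBP_PlayerGameUI, whose only ShowGameUI call is unreachable.
; UseObject calls AddWBPTicket, sets the widget's Message and returns false.
; AddWBPTicket switches input to the Puzzle profile, makes the player capsule ignore Visibility traces and adds the widget to the viewport.
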(event `self.ReceiveBeginPlay`
  (`parent.ReceiveBeginPlay`)
  (bind _returnvalue (`|CreateWidget` "/Game/Blueprint/Tickets/WBP_Ticket.WBP_Ticket_C"))
  (set `self.WBP_TicketRefer` _returnvalue)
  (bind _returnvalue_2 (`|CreateWidget` "/Game/PNCTookit/Blueprints/Widgets/Gameplay/WBP_PlayerGameUI.WBP_PlayerGameUI_C"))
  (set `self.WBP_PlayerGameRefer` _returnvalue_2))

(fn `AddWBP_Ticket`
  (`/Game/PNCTookit/Blueprints/BP_PNCPlayerController.SetInputProfile` (`/Game/PNCTookit/Blueprints/FunctionLibraries/BPFL_Controller.GetPNC_PlayerController`) "Puzzle")
  (`PrimitiveComponent.SetCollisionResponseToChannel` (`Character.CapsuleComponent` (`/Game/PNCTookit/Blueprints/FunctionLibraries/BPFL_Controller.GetPNC_Character`)) "ECC_Visibility" "ECR_Ignore")
  (`UserWidget.AddToViewport` (`self.WBP_TicketRefer`) 0))

(fn `UseObject`
  (params (InteractingCharacter :type "/Game/PNCTookit/Blueprints/Characters/BP_PNCCharacter_Parent Object Reference"))
  (returns (Success :type Boolean))
  (`self.AddWBP_Ticket`)
  (set `/Game/Blueprint/Tickets/WBP_Ticket.Message` (`self.Message`) (`self.WBP_TicketRefer`))
  (return false))

(fn `UserConstructionScript`
  (`parent.UserConstructionScript`))