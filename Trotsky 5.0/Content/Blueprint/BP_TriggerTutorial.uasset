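; BP_TriggerTutorial is a trigger volume that shows a one-time tutorial popup with configurable text.
; BeginPlay creates a WBP_Tutorial widget and fills in its text; the first box overlap adds it to the viewport and binds its button to close it.
; While shown, the player controller uses the Puzzle input profile and the character capsule ignores Visibility traces; closing restores Gameplay input and blocking.
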(event `self.ReceiveBeginPlay`
  (bind _returnvalue (`|CreateWidget` "/Game/Blueprint/Widgets/WBP_Tutorial.WBP_Tutorial_C"))
  (set `self.WBP_TutorialRefer` _returnvalue)
  (set `/Game/Blueprint/Widgets/WBP_Tutorial.TextTutorial` (`self.Tutorial Text`) (`self.WBP_TutorialRefer`)))

(event `self.Box.OnComponentBeginOverlap`
  (params (OverlappedComponent :type "PrimitiveComponent Object Reference") (OtherActor :type "Actor Object Reference") (OtherComp :type "PrimitiveComponent Object Reference") (OtherBodyIndex :type Integer) (bFromSweep :type Boolean) (SweepResult :type "HitResult Structure (by ref)"))
  (`/Engine/EditorBlueprintResources/StandardMacros.DoOnce` false
    (:`Completed`
      (`self.AddWidget`)
      (add `Button.OnClicked` (`/Game/Blueprint/Widgets/WBP_Tutorial.Button_232` (`self.WBP_TutorialRefer`)) (delegate `RemoveWidget`)))))

(event `RemoveWidget`
  (`self.RemoveWidge`))

(fn `AddWidget`
  (`/Game/PNCTookit/Blueprints/BP_PNCPlayerController.SetInputProfile` (`/Game/PNCTookit/Blueprints/FunctionLibraries/BPFL_Controller.GetPNC_PlayerController`) "Puzzle")
  (`PrimitiveComponent.SetCollisionResponseToChannel` (`Character.CapsuleComponent` (`/Game/PNCTookit/Blueprints/FunctionLibraries/BPFL_Controller.GetPNC_Character`)) "ECC_Visibility" "ECR_Ignore")
  (`UserWidget.AddToViewport` (`self.WBP_TutorialRefer`) 0))

(fn `RemoveWidge`
  (`Widget.RemoveFromParent` (`self.WBP_TutorialRefer`))
  (`/Game/PNCTookit/Blueprints/BP_PNCPlayerController.SetInputProfile` (`/Game/PNCTookit/Blueprints/FunctionLibraries/BPFL_Controller.GetPNC_PlayerController`) "Gameplay")
  (`PrimitiveComponent.SetCollisionResponseToChannel` (`Character.CapsuleComponent` (`/Game/PNCTookit/Blueprints/FunctionLibraries/BPFL_Controller.GetPNC_Character`)) "ECC_Visibility" "ECR_Block"))

(fn `UserConstructionScript`)