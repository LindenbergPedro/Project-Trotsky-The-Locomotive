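; Scene manager Blueprint for level 01, containing an example scripted camera cutscene.
; BeginExampleCutscene disables PNC player input, cuts between two cutscene cameras with timed delays, then eases the view back to the PNC camera manager.
; Input is re-enabled as that final blend starts, without waiting for it to finish.
; The event graph and construction script add no logic of their own.
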(event `BeginExampleCutscene`
  ;[1 1 1] Example Cutscene
  (`/Game/PNCTookit/Blueprints/BP_PNCPlayerController.SetInputEnabled` (`/Game/PNCTookit/Blueprints/FunctionLibraries/BPFL_Controller.GetPNC_PlayerController`) false)
  (`PlayerController.SetViewTargetWithBlend` (`/Game/PNCTookit/Blueprints/FunctionLibraries/BPFL_Controller.GetPNC_PlayerController`) (`self.ExampleCutsceneCamera1`) 0.0 "VTBlend_Linear" 0.0 false)
  (`KismetSystemLibrary.Delay` 3.0)
  (`PlayerController.SetViewTargetWithBlend` (`/Game/PNCTookit/Blueprints/FunctionLibraries/BPFL_Controller.GetPNC_PlayerController`) (`self.ExampleCutsceneCamera2`) 0.0 "VTBlend_Linear" 0.0 false)
  (`KismetSystemLibrary.Delay` 3.0)
  (`PlayerController.SetViewTargetWithBlend` (`/Game/PNCTookit/Blueprints/FunctionLibraries/BPFL_Controller.GetPNC_PlayerController`) (`/Game/PNCTookit/Blueprints/FunctionLibraries/BPFL_Controller.GetPNC_CameraManager`) 1.0 "VTBlend_EaseInOut" 5.0 false)
  (`/Game/PNCTookit/Blueprints/BP_PNCPlayerController.SetInputEnabled` (`/Game/PNCTookit/Blueprints/FunctionLibraries/BPFL_Controller.GetPNC_PlayerController`) true))

(fn `UserConstructionScript`
  (`parent.UserConstructionScript`))