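; Vodka item pickup that can only be taken once the cabinet-broken flag (ArmarioQuebrado) is set.
; When the flag is set, Pickup plays a sound, sets HasVodka, hides the mesh, disables mesh and sphere collision, and returns true.
; Otherwise it plays another sound and calls Dialogo_quebrado to start the "Pegarnotvodka" dialogue sequence.
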(event `self.ReceiveBeginPlay`
  (`parent.ReceiveBeginPlay`))

(event `Dialogo_quebrado`
  (`/Game/PNCTookit/Blueprints/FunctionLibraries/BPFL_Dialogue.StartDialogueSequence` "Pegarnotvodka" self))

(fn `Pickup`
  (params (Instigator :type "Actor Object Reference"))
  (returns (Success :type Boolean))
  (if (`self.ArmarioQuebrado`)
    (`GameplayStatics.PlaySound2D` "/Game/Audio/Açoes/Pegar_Item.Pegar_Item" 1.0 1.0 0.0 null null)
    (bind _output_get (set `self.HasVodka` true))
    (`SceneComponent.SetVisibility` (`self.StaticMesh`) (not _output_get) false)
    (`PrimitiveComponent.SetCollisionEnabled` (`self.Sphere`) "NoCollision")
    (`PrimitiveComponent.SetCollisionEnabled` (`self.StaticMesh`) "NoCollision")
    (return true)
    (else
      (`GameplayStatics.PlaySound2D` "/Game/Audio/Açoes/Abrir_carta.Abrir_carta" 1.0 1.0 0.0 null null)
      (`self.Dialogo_quebrado`))))

(fn `UserConstructionScript`
  (`parent.UserConstructionScript`))