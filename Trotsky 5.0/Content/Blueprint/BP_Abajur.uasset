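; BP_Abajur is an interactable lamp (abajur) that the player can switch on and off.
; Its UseObject override runs the parent logic first and, if that succeeds, flips IsUsed and calls LightOn or LightOff to show or hide the PointLight.
; BeginPlay creates a WBP_LookAndPick widget and caches it along with a reference to the BP_PNCCharacter_3D_Player actor.
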(event `self.ReceiveBeginPlay`
  (`parent.ReceiveBeginPlay`)
  (bind _returnvalue (`|CreateWidget` "/Game/Blueprint/Widgets/WBP_LookAndPick.WBP_LookAndPick_C" (`GameplayStatics.GetPlayerController` 0)))
  (set `self.WBP_LookRefer` _returnvalue)
  (bind _returnvalue_2 (`GameplayStatics.GetActorOfClass` "/Game/PNCTookit/Blueprints/Characters/3D/BP_PNCCharacter_3D_Player.BP_PNCCharacter_3D_Player_C"))
  (set `self.CharacterRefer` _returnvalue_2))

(event `LightOn`
  (`SceneComponent.SetVisibility` (`self.PointLight`) true false))

(event `LightOff`
  (`SceneComponent.SetVisibility` (`self.PointLight`) false false))

(fn `UseObject`
  (params (InteractingCharacter :type "/Game/PNCTookit/Blueprints/Characters/BP_PNCCharacter_Parent Object Reference"))
  (returns (Success :type Boolean))
  (bind _success (`parent.UseObject` InteractingCharacter))
  (if _success
    (if (`self.bIsUsed`)
      (set `self.bIsUsed` false)
      (`self.LightOff`)
      (else
        (set `self.bIsUsed` true)
        (`self.LightOn`))))
  (return _success))

(fn `UserConstructionScript`
  (`parent.UserConstructionScript`))