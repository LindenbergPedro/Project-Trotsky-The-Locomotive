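; Player controller for Jehan that handles click-to-move, a context-sensitive mouse cursor and pausing.
; On BeginPlay the local controller sets game-and-UI input, views its pawn and installs a UIMouseModes widget on the EyeDropper cursor slot.
; SetDestination sends the cursor's visibility-trace hit location to the character's MoveToLocation.
; SetMouseContext forwards context and chance to the cursor widget, cursor-over events switch context, and Pause opens UIPause.
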(event `self.ReceiveBeginPlay`
  (if (`self.IsLocalPlayerController`)
    (`WidgetBlueprintLibrary.SetInputMode_GameAndUIEx` self null "DoNotLock" false)
    (`self.SetViewTargetWithBlend` (`self.K2_GetPawn`))
    (bind _returnvalue (`|CreateWidget` "/Game/Interface/UI-MouseModes.UI-MouseModes_C"))
    (bind _output_get (set `self.CursorRef` _returnvalue))
    (`self.SetMouseCursorWidget` "EyeDropper" _output_get)
    (set `self.bShowMouseCursor` true)))

(event `/Game/Blueprint/MouseModes/BPI_ContextMouseInterface.SetMouseContext`
  (params (Context :type "/Game/Blueprint/MouseModes/E_CursorModes Enum" :default "NewEnumerator0") (ShowChance :type Boolean) (Chance :type Integer))
  (message `/Game/Blueprint/MouseModes/BPI_ContextMouseInterface.SetMouseContext` (`self.CursorRef`) Context ShowChance Chance))

(event `InputAction|SetDestination`
  (params (Key :type "Key Structure"))
  ;[1 1 1] Movemnet
  (:`Pressed`
    (bind _asbp_character_jehan (cast `/Game/Blueprint/BP_Character_Jehan` (`GameplayStatics.GetPlayerCharacter` 0)))
    (`/Game/Blueprint/BP_Character_Jehan.MoveToLocation` _asbp_character_jehan (`.Location` (`GameplayStatics.BreakHitResult` (`self.GetHitResultUnderCursorByChannel` "TraceTypeQuery1"))))))

(event `self.ReceiveActorBeginCursorOver`
  (message `/Game/Blueprint/MouseModes/BPI_ContextMouseInterface.SetMouseContext` (`GameplayStatics.GetPlayerController` 0) "NewEnumerator3" false 0))

(event `InputAction|Pause`
  (params (Key :type "Key Structure"))
  (:`Pressed`
    (`GameplayStatics.SetGamePaused` true)
    (bind _returnvalue (`|CreateWidget` "/Game/Interface/UI-Pause.UI-Pause_C"))
    (`UserWidget.AddToViewport` _returnvalue 0)))

(event `self.ReceiveActorEndCursorOver`
  (message `/Game/Blueprint/MouseModes/BPI_ContextMouseInterface.SetMouseContext` (`GameplayStatics.GetPlayerController` 0) "NewEnumerator1" false 0))

(fn `UserConstructionScript`)