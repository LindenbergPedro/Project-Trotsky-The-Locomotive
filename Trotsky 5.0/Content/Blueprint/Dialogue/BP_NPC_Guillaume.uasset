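; Guillaume, an interactable dialogue NPC who can reveal an item, apparently a key, depending on the drink state.
; Construction passes his tag and display name to the interaction component and positions the dialogue point.
; Using him starts his dialogue row; he rejects all offered items.
; The Spawn.key dialogue option activates the referenced item if the level's BP_Drink has HasDrink set, otherwise plays a fallback dialogue.
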(fn `OnReturnDialogueOption`
  (params (ReturnOption :type String))
  (returns (Success :type Boolean))
  (switch `string` ReturnOption
    (:`spawn.key`
      (bind _returnvalue (`GameplayStatics.GetActorOfClass` "/Game/Blueprint/Drinks/BP_Drink.BP_Drink_C"))
      (if (`/Game/Blueprint/Drinks/BP_Drink.HasDrink` _returnvalue)
        (`/Game/PNCTookit/Blueprints/Gameplay/Items/BP_ItemBase.SetItemActiveState` (`self.ItemRef`) true)
        (return true)
        (else
          (`/Game/PNCTookit/Blueprints/FunctionLibraries/BPFL_Dialogue.StartDialogueSequence` "Guillaume_03" self))))))

(fn `RecieveItem`
  (params (ItemName :type Name))
  (returns (Valid :type Boolean) (Consumed :type Boolean))
  (return false false))

(fn `UseObject`
  (params (InteractingCharacter :type "/Game/PNCTookit/Blueprints/Characters/BP_PNCCharacter_Parent Object Reference"))
  (returns (Success :type Boolean))
  (bind _success (`parent.UseObject` InteractingCharacter))
  (if _success
    (`/Game/PNCTookit/Blueprints/FunctionLibraries/BPFL_Dialogue.StartDialogueSequence` (`self.Dialogue Row Name`) self)
    (return false)))

(fn `UserConstructionScript`
  (bind _globalinteractioncomponent (`self.GlobalInteractionComponent`))
  (set `/Game/PNCTookit/Blueprints/Components/BP_GlobalInteractionComponent.GameplayTag` (`self.Gameplay Tag`) _globalinteractioncomponent)
  (set `/Game/PNCTookit/Blueprints/Components/BP_GlobalInteractionComponent.DisplayName` (`self.NomeNPC`) _globalinteractioncomponent)
  (`SceneComponent.K2_SetRelativeLocation` (`self.DialoguePositionSceneComponent`) (`self.LocationDialogue`) false false)
  (`parent.UserConstructionScript`))