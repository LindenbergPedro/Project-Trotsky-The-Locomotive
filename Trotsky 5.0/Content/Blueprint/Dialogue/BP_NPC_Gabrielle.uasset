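; Gabrielle NPC Blueprint that opens a dialogue sequence when used, provided the parent's use check passes.
; Construction copies the gameplay tag and NPC name into the global interaction component and positions the dialogue scene component.
; Returned dialogue options spawn particles beside the actor: fire for "Particle Fire", a leaf effect for "Particle Smoke".
; Items offered to the NPC are always rejected as invalid and not consumed.
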(fn `OnReturnDialogueOption`
  (params (ReturnOption :type String))
  (returns (Success :type Boolean))
  (bind _returnvalue (+ (`self.K2_GetActorLocation`) (-50.0 0.0 0.0)))
  (switch `string` ReturnOption
    (:`particle_fire`
      (`GameplayStatics.SpawnEmitterAtLocation` "/Game/PNCTookit/PNCGame/Scenes/Shared/Effects/P_Fire.P_Fire" _returnvalue (struct) (0.5 0.5 0.5)))
    (:`particle_smoke`
      (`GameplayStatics.SpawnEmitterAtLocation` "/Game/PNCTookit/PNCGame/Scenes/Shared/Effects/P_Leaf.P_Leaf" _returnvalue)))
  (return true))

(fn `RecieveItem`
  (params (ItemName :type Name))
  (returns (Valid :type Boolean) (Consumed :type Boolean))
  (return false false))

(fn `UseObject`
  (params (InteractingCharacter :type "/Game/PNCTookit/Blueprints/Characters/BP_PNCCharacter_Parent Object Reference"))
  (returns (Success :type Boolean))
  (bind _success (`parent.UseObject` InteractingCharacter))
  (if _success
    (`/Game/PNCTookit/Blueprints/FunctionLibraries/BPFL_Dialogue.StartDialogueSequence` (`self.Dialogue Row Name`) self)
    (return false)))

(fn `UserConstructionScript`
  (bind _globalinteractioncomponent (`self.GlobalInteractionComponent`))
  (set `/Game/PNCTookit/Blueprints/Components/BP_GlobalInteractionComponent.GameplayTag` (`self.Gameplay Tag`) _globalinteractioncomponent)
  (set `/Game/PNCTookit/Blueprints/Components/BP_GlobalInteractionComponent.DisplayName` (`self.NomeNPC`) _globalinteractioncomponent)
  (`SceneComponent.K2_SetRelativeLocation` (`self.DialoguePositionSceneComponent`) (`self.LocationDialogue`) false false)
  (`parent.UserConstructionScript`))