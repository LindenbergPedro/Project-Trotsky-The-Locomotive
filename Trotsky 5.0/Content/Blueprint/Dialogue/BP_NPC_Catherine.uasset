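; Interactable dialogue NPC Catherine, whose Drink dialogue option opens the WBP_Drink screen.
; UseObject starts the configured dialogue row, while the ActiveDrink event starts its own row.
; The widget is created at BeginPlay; showing it switches to Puzzle input and UI-only mode, and RemoveWBPDrink restores gameplay input.
; The Caipiroska activation and widget removal in the option handler are disconnected and never run.
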(event `self.ReceiveBeginPlay`
  (bind _returnvalue (`|CreateWidget` "/Game/Blueprint/Widgets/WBP_Drink.WBP_Drink_C" (`GameplayStatics.GetPlayerController` 0)))
  (set `self.WBP_DrinkRefer` _returnvalue))

(event `ActiveDrink`
  (`/Game/PNCTookit/Blueprints/FunctionLibraries/BPFL_Dialogue.StartDialogueSequence` "ActiveDrink" self))

(fn `AddWBP_Drink`
  (bind _wbp_drinkrefer (`self.WBP_DrinkRefer`))
  (`/Game/PNCTookit/Blueprints/BP_PNCPlayerController.SetInputProfile` (`/Game/PNCTookit/Blueprints/FunctionLibraries/BPFL_Controller.GetPNC_PlayerController`) "Puzzle")
  (`PrimitiveComponent.SetCollisionResponseToChannel` (`Character.CapsuleComponent` (`/Game/PNCTookit/Blueprints/FunctionLibraries/BPFL_Controller.GetPNC_Character`)) "ECC_Visibility" "ECR_Ignore")
  (`UserWidget.AddToViewport` _wbp_drinkrefer 0)
  (`WidgetBlueprintLibrary.SetInputMode_UIOnlyEx` (`GameplayStatics.GetPlayerController` 0) _wbp_drinkrefer))

(fn `OnReturnDialogueOption`
  (params (ReturnOption :type String))
  (returns (Success :type Boolean))
  (switch `string` ReturnOption
    (:`drink`
      (`self.AddWBP_Drink`)
      (return true))))

(fn `RemoveWBP_Drink`
  (`Widget.RemoveFromParent` (`self.WBP_DrinkRefer`))
  (`/Game/PNCTookit/Blueprints/BP_PNCPlayerController.SetInputProfile` (`/Game/PNCTookit/Blueprints/FunctionLibraries/BPFL_Controller.GetPNC_PlayerController`) "Gameplay")
  (`self.SetActorHiddenInGame` (`/Game/PNCTookit/Blueprints/FunctionLibraries/BPFL_Controller.GetPNC_Character`) false)
  (`PrimitiveComponent.SetCollisionResponseToChannel` (`Character.CapsuleComponent` (`/Game/PNCTookit/Blueprints/FunctionLibraries/BPFL_Controller.GetPNC_Character`)) "ECC_Visibility" "ECR_Block")
  (`WidgetBlueprintLibrary.SetInputMode_GameAndUIEx` (`GameplayStatics.GetPlayerController` 0) (`self.WBP_DrinkRefer`)))

(fn `UseObject`
  (params (InteractingCharacter :type "/Game/PNCTookit/Blueprints/Characters/BP_PNCCharacter_Parent Object Reference"))
  (returns (Success :type Boolean))
  (bind _success (`parent.UseObject` InteractingCharacter))
  (if _success
    (`/Game/PNCTookit/Blueprints/FunctionLibraries/BPFL_Dialogue.StartDialogueSequence` (`self.Dialogue Row Name`) self)
    (return false)))

(fn `UserConstructionScript`
  (bind _globalinteractioncomponent (`self.GlobalInteractionComponent`))
  (set `/Game/PNCTookit/Blueprints/Components/BP_GlobalInteractionComponent.GameplayTag` (`self.Gameplay Tag`) _globalinteractioncomponent)
  (set `/Game/PNCTookit/Blueprints/Components/BP_GlobalInteractionComponent.DisplayName` (`self.NomeNPC`) _globalinteractioncomponent)
  (`SceneComponent.K2_SetRelativeLocation` (`self.DialoguePositionSceneComponent`) (`self.LocationDialogue`) false false)
  (`parent.UserConstructionScript`))