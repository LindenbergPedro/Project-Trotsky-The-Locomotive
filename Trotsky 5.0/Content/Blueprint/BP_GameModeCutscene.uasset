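; Game mode Blueprint for the intro cutscene, narrating in Portuguese Jehan the art thief boarding the Trotsky train to steal the painting La comuna.
; On BeginPlay it plays sound and adds the WB_Cutscene01 widget to the viewport.
; A fixed chain of delays updates the widget text line by line, each with a sound.
; It then clears the text, plays a last sound and opens Level01.
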(event `self.ReceiveBeginPlay`
  ;[1 1 1] Som de fundo
  (`GameplayStatics.PlaySound2D` null 1.0 1.0 0.0 null null)
  (bind _returnvalue (`|CreateWidget` "/Game/Blueprint/Cutscenes/WB_Cutscene01.WB_Cutscene01_C"))
  (bind _output_get (set `self.WB_CutsceneRefer` _returnvalue))
  (`UserWidget.AddToViewport` _output_get 0)
  (`KismetSystemLibrary.Delay` 1.0)
  (`GameplayStatics.PlaySound2D` null 1.0 1.0 0.0 null null)
  (`/Game/Blueprint/Cutscenes/WB_Cutscene01.UpdateText` (`self.WB_CutsceneRefer`) "A La comuna é uma obra de arte com mais de 500 anos.")
  (`KismetSystemLibrary.Delay` 4.0)
  (`GameplayStatics.PlaySound2D` null 1.0 1.0 0.0 null null)
  (`/Game/Blueprint/Cutscenes/WB_Cutscene01.UpdateText` (`self.WB_CutsceneRefer`) "Está sendo transportada pela locomotiva Trotsky até o festival de belas artes.")
  (`KismetSystemLibrary.Delay` 5.0)
  (`GameplayStatics.PlaySound2D` null 1.0 1.0 0.0 null null)
  (`/Game/Blueprint/Cutscenes/WB_Cutscene01.UpdateText` (`self.WB_CutsceneRefer`) "Jehan, o famoso ladrão de artes, embarcou no Trem Trotsky, com o desejo de tentar roubar a La comuna.")
  (`KismetSystemLibrary.Delay` 5.0)
  (`GameplayStatics.PlaySound2D` null 1.0 1.0 0.0 null null)
  (`/Game/Blueprint/Cutscenes/WB_Cutscene01.UpdateText` (`self.WB_CutsceneRefer`) "Mal sabe ele que grandes perigos rondam à locomotiva Trotsky.")
  (`KismetSystemLibrary.Delay` 4.0)
  (`/Game/Blueprint/Cutscenes/WB_Cutscene01.ClearText` (`self.WB_CutsceneRefer`))
  (`GameplayStatics.PlaySound2D` null 1.0 1.0 0.0 null null)
  (`KismetSystemLibrary.Delay` 4.0)
  (`GameplayStatics.OpenLevel` "Level01"))

(fn `UserConstructionScript`)