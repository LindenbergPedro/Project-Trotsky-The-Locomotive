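; BP_Menu3D is a 3D menu actor that hosts a UI-Menu3D widget and moves the player's view between linked menus.
; On BeginPlay it binds to the widget's TransitionToLinkedMenu dispatcher and disables its own collision.
; The dispatched index selects a LinkedMenus entry, which becomes player 0's view target through an eased camera blend.
; Each transition also switches collision off on the current menu and on for the destination.
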(event `self.ReceiveBeginPlay`
  ;[1 1 1] Criação do widget
  (bind _asui_menu_3d (cast `/Game/Interface/Menu/UI-Menu3D` (`WidgetComponent.GetUserWidgetObject` (`self.Widget`))))
  (add `/Game/Interface/Menu/UI-Menu3D.TransitionToLinkedMenu` _asui_menu_3d (delegate `OnTransitionBetweenMenus`))
  (`self.SetActorEnableCollision` false))

(event `OnTransitionBetweenMenus`
  (params (MenuIndex :type Integer))
  ;[1 1 1] Criação do widget
  (if (`KismetArrayLibrary.Array_IsValidIndex` (`self.LinkedMenus`) MenuIndex)
    (`self.TransitionTO` (`|GetArrayItem` (`self.LinkedMenus`) MenuIndex))))

(event `TransitionTO`
  (params (NewMenu :type "/Game/Blueprint/Menu/BP_Menu3D Object Reference"))
  ;[1 1 1] Transação da Camera
  (`self.SetActorEnableCollision` false)
  (`self.SetActorEnableCollision` NewMenu true)
  (`PlayerController.SetViewTargetWithBlend` (`GameplayStatics.GetPlayerController` 0) NewMenu 2.0 "VTBlend_EaseInOut" 2.0 false))

(fn `UserConstructionScript`)