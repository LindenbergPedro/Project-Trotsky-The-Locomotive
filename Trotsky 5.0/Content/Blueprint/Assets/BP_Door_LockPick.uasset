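; Interactable door that opens and closes on use, typed as lock-pick, key or open.
; UseObject checks the key or lock-pick tool; lock-pick doors show dialogue without the tool, or the WBP_LookAndPick puzzle widget under a Puzzle input profile until unlocked.
; A timeline slides or rotates the door mesh, reversing to close.
; Sliding doors also toggle optional curtain and roof actors as the timeline updates.
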(event `self.ReceiveBeginPlay`
  (`parent.ReceiveBeginPlay`)
  (bind _returnvalue (`|CreateWidget` "/Game/Blueprint/Widgets/WBP_LookAndPick.WBP_LookAndPick_C" (`GameplayStatics.GetPlayerController` 0)))
  (set `self.WBP_LookRefer` _returnvalue)
  (bind _returnvalue_2 (`GameplayStatics.GetActorOfClass` "/Game/PNCTookit/Blueprints/Characters/3D/BP_PNCCharacter_3D_Player.BP_PNCCharacter_3D_Player_C"))
  (set `self.CharacterRefer` _returnvalue_2))

(event `OpenDoor`
  (set `self.DoorOpen?` true)
  (`AddComponent|NODE_AddAudioComponent-2`)
  (bind (_direction _alpha) (`Timeline|Timeline_0` :!via `PlayFromStart` :!label _label)
    (:`Update`
      (if (`self.Sliding or rotation`)
        ;[1 1 1] Set Visivle Curtain and Roof
        (`self.SetVisibleCurtain`)
        (`self.SetVisibleRoof`)
        ;[1 1 1] Open Door Sliding
        (`SceneComponent.K2_SetRelativeLocation` (`self.CBN_locomotive_door`) (`KismetMathLibrary.VLerp` (0.0 0.0 0.0) (`self.TransleterOpen`) _alpha) false false)
        (else
          ;[1 1 1] Open Door Rotation
          (`SceneComponent.K2_SetRelativeRotation` (`self.CBN_locomotive_door`) (`KismetMathLibrary.RLerp` (struct) (struct :`Yaw` -120.0) _alpha) false false))))))

(event `CloseDoor`
  (set `self.DoorOpen?` false)
  (`GameplayStatics.PlaySound2D` "/Game/Audio/Açoes/Door_Sliding_-_Open.Door_Sliding_-_Open" 1.0 1.0 0.0 null null)
  (goto _label :!via `ReverseFromEnd`))

(fn `AddMenuLook`
  (`/Game/PNCTookit/Blueprints/BP_PNCPlayerController.SetInputProfile` (`/Game/PNCTookit/Blueprints/FunctionLibraries/BPFL_Controller.GetPNC_PlayerController`) "Puzzle")
  (`PrimitiveComponent.SetCollisionResponseToChannel` (`Character.CapsuleComponent` (`/Game/PNCTookit/Blueprints/FunctionLibraries/BPFL_Controller.GetPNC_Character`)) "ECC_Visibility" "ECR_Ignore")
  (`UserWidget.AddToViewport` (`self.WBP_LookRefer`) 0))

(fn `RemoveMenuLook`
  (`Widget.RemoveFromParent` (`self.WBP_LookRefer`))
  (`/Game/PNCTookit/Blueprints/BP_PNCPlayerController.SetInputProfile` (`/Game/PNCTookit/Blueprints/FunctionLibraries/BPFL_Controller.GetPNC_PlayerController`) "Gameplay")
  (`self.SetActorHiddenInGame` (`/Game/PNCTookit/Blueprints/FunctionLibraries/BPFL_Controller.GetPNC_Character`) false)
  (`PrimitiveComponent.SetCollisionResponseToChannel` (`Character.CapsuleComponent` (`/Game/PNCTookit/Blueprints/FunctionLibraries/BPFL_Controller.GetPNC_Character`)) "ECC_Visibility" "ECR_Block"))

(fn `SetVisibleCurtain`
  (bind _curtainopen (`self.CurtainOpen`))
  (bind _curtainclosed (`self.CurtainClosed`))
  (if (`self.HasCurtain?`)
    (if (`self.DoorOpen?`)
      (`self.SetActorHiddenInGame` _curtainclosed true)
      (`self.SetActorHiddenInGame` _curtainopen false)
      (`self.SetActorEnableCollision` _curtainclosed false)
      (else
        (`self.SetActorHiddenInGame` _curtainclosed false)
        (`self.SetActorHiddenInGame` _curtainopen true)
        (`self.SetActorEnableCollision` _curtainclosed true))))
  (return))

(fn `SetVisibleRoof`
  (bind _roof (`self.Roof`))
  (if (`self.HasRoof?`)
    (if (`self.DoorOpen?`)
      (`self.SetActorHiddenInGame` _roof true)
      (else
        (`self.SetActorHiddenInGame` _roof false))))
  (return))

(fn `UseObject`
  (params (InteractingCharacter :type "/Game/PNCTookit/Blueprints/Characters/BP_PNCCharacter_Parent Object Reference"))
  (returns (Success :type Boolean))
  (bind _success (`parent.UseObject` InteractingCharacter))
  (switch `/Game/Blueprint/Assets/Enum_TypesDoor` (`self.TypesDoor`)
    (:`NewEnumerator0`
      (bind _returnvalue (`GameplayStatics.GetActorOfClass` "/Game/Blueprint/Itens/BP_Ferramentas.BP_Ferramentas_C"))
      (if (`/Game/Blueprint/Itens/BP_Ferramentas.HasLockPick` _returnvalue)
        (if (`/Game/Blueprint/Widgets/WBP_LookAndPick.Unlocked?` (`self.WBP_LookRefer`))
          (if _success :!label _label
            (if (`self.bIsUsed`)
              (set `self.bIsUsed` false)
              (`self.CloseDoor`)
              (else
                (set `self.bIsUsed` true)
                (`self.OpenDoor`))))
          (return _success)
          (else
            (`|ExecutionSequence`
              (:`then_1`
                (`self.AddMenuLook`)
                (if (`/Game/Blueprint/Widgets/WBP_LookAndPick.Unlocked?` (`self.WBP_LookRefer`))
                  (`self.RemoveMenuLook`))))))
        (else
          (`/Game/PNCTookit/Blueprints/FunctionLibraries/BPFL_Dialogue.StartDialogueSequence` "Door_LockPick" self))))
    (:`NewEnumerator1`
      (bind _returnvalue_2 (`GameplayStatics.GetActorOfClass` "/Game/Blueprint/Itens/BP_Key2.BP_Key2_C"))
      (if (`/Game/Blueprint/Itens/BP_Key2.HasKey` _returnvalue_2)
        (goto _label)))
    (:`NewEnumerator2`
      (goto _label))))

(fn `UserConstructionScript`
  (`parent.UserConstructionScript`))