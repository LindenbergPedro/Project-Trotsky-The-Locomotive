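; BP_Maleta2 is a usable suitcase ("maleta") that is locked behind a coded puzzle.
; When IsOpen is set, UseObject starts the puzzle while locked, and a successful result sets Unlocked.
; Once unlocked, each use plays or reverses a timeline that rotates the lid.
; The same toggle switches the item active state of the BP_Ferramentas (tools) actor found at BeginPlay.
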(event `self.ReceiveBeginPlay`
  (`parent.ReceiveBeginPlay`)
  (bind _returnvalue (`GameplayStatics.GetActorOfClass` "/Game/Blueprint/Itens/BP_Ferramentas.BP_Ferramentas_C"))
  (set `self.FerramentasRefer` _returnvalue))

(event `OpenMaleta`
  (bind (_direction _alpha) (`Timeline|OpenTimeline` :!via `PlayFromStart` :!label _label)
    (:`Update`
      (`SceneComponent.K2_SetRelativeRotation` (`self.Top`) (`KismetMathLibrary.RLerp` (struct :`Roll` 90.0) (struct) _alpha) false false))))

(event `CloseMaleta`
  (goto _label :!via `ReverseFromEnd`))

(fn `ReturnPuzzleResult`
  (params (Success :type Boolean))
  (returns (Return :type Boolean))
  (if Success
    (set `self.Unlocked` true))
  (return false))

(fn `UseObject`
  (params (InteractingCharacter :type "/Game/PNCTookit/Blueprints/Characters/BP_PNCCharacter_Parent Object Reference"))
  (returns (Success :type Boolean))
  (bind _ferramentasrefer (`self.FerramentasRefer`))
  (if (`self.IsOpen`)
    (if (`self.Unlocked`)
      (if (`self.bIsUsed`)
        (set `self.bIsUsed` false)
        (`self.CloseMaleta`)
        (`/Game/PNCTookit/Blueprints/Gameplay/Items/BP_ItemBase.SetItemActiveState` _ferramentasrefer false)
        (else
          (set `self.bIsUsed` true)
          (`self.OpenMaleta`)
          (`/Game/PNCTookit/Blueprints/Gameplay/Items/BP_ItemBase.SetItemActiveState` _ferramentasrefer true)))
      (return false)
      (else
        (`/Game/PNCTookit/Blueprints/Gameplay/Puzzles/BPFL_PuzzleHelpers.StartPuzzle` "NewEnumerator4" self 1947)))))

(fn `UserConstructionScript`
  (`parent.UserConstructionScript`))