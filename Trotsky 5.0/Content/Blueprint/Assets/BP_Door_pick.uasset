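; BP_Door_pick is a key-locked interactable door that either slides or swings open.
; Its UseObject override calls the parent, then requires HasKey on the BP_Key2 found in the level, CanOpen and a true parent result before toggling IsUsed.
; One timeline plays forward to open and reverses to close, lerping CBNLocomotiveDoor's relative location or rotation according to SlidingOrRotation.
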(event `OpenDoor`
  (bind (_direction _alpha) (`Timeline|Timeline_0` :!via `PlayFromStart` :!label _label)
    (:`Update`
      (if (`self.Sliding or rotation`)
        ;[1 1 1] Open Door Sliding
        (`SceneComponent.K2_SetRelativeLocation` (`self.CBN_locomotive_door`) (`KismetMathLibrary.VLerp` (0.0 0.0 0.0) (`self.TransleterOpen`) _alpha) false false)
        (else
          ;[1 1 1] Open Door Rotation
          (`SceneComponent.K2_SetRelativeRotation` (`self.CBN_locomotive_door`) (`KismetMathLibrary.RLerp` (struct) (struct :`Yaw` -75.0) _alpha) false false))))))

(event `CloseDoor`
  (goto _label :!via `ReverseFromEnd`))

(fn `UseObject`
  (params (InteractingCharacter :type "/Game/PNCTookit/Blueprints/Characters/BP_PNCCharacter_Parent Object Reference"))
  (returns (Success :type Boolean))
  (bind _success (`parent.UseObject` InteractingCharacter))
  (bind _returnvalue (`GameplayStatics.GetActorOfClass` "/Game/Blueprint/Itens/BP_Key2.BP_Key2_C"))
  (if (`/Game/Blueprint/Itens/BP_Key2.HasKey` _returnvalue)
    (if (`self.CanOpen?`)
      (if _success
        (if (`self.bIsUsed`)
          (set `self.bIsUsed` false)
          (`self.CloseDoor`)
          (else
            (set `self.bIsUsed` true)
            (`self.OpenDoor`))))
      (return _success))))

(fn `UserConstructionScript`
  (`parent.UserConstructionScript`))