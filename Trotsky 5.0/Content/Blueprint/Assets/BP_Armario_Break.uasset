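; Interactable cabinet that the player breaks by giving it the "Ferro" item.
; Using it toggles a used flag, playing the "Armario" dialogue on every other use starting with the second, and it cannot be picked up.
; Receiving Ferro adds it to the inventory component and, on success, destroys the intact mesh, reveals the broken one and flags the parent BP_Vodka actor.
; The opening sound is disconnected and never plays.
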(event `Clicavel`
  (`/Game/PNCTookit/Blueprints/FunctionLibraries/BPFL_Dialogue.StartDialogueSequence` "Armario" self))

(fn `GetItemName`
  (returns (NewParam :type Name))
  (return "None"))

(fn `IsInventoryItem`
  (returns (return :type Boolean))
  (return false))

(fn `OnInspection `
  (params (Inspector :type "Controller Object Reference"))
  (returns (Success :type Boolean))
  (return false))

(fn `Pickup`
  (params (Instigator :type "Actor Object Reference"))
  (returns (Success :type Boolean))
  (return false))

(fn `RecieveItem`
  (params (ItemName :type Name))
  (returns (Valid :type Boolean) (Consumed :type Boolean))
  (switch `name` ItemName
    (:`Default`
      (return false false))
    (:`Ferro`
      (bind _return (`/Game/PNCTookit/Blueprints/Components/BP_InventoryComponent.AddInventoryItem` (`self.BP_InventoryComponent`) "Ferro"))
      (`self.TrocaMesh` _return)
      (return _return _return))))

(fn `TrocaMesh`
  (params (bIsActive :type Boolean))
  (bind _output_get (set `self.bIsActive` bIsActive))
  (if _output_get
    (`ActorComponent.K2_DestroyComponent` (`self.Mesh_Inteira`))
    (`SceneComponent.SetVisibility` (`self.Mesh_quebrada`) true false)
    (bind _asbp_vodka (cast `/Game/Blueprint/Itens/BP_Vodka` (`self.GetParentActor`)))
    (set `/Game/Blueprint/Itens/BP_Vodka.ArmarioQuebrado` true _asbp_vodka)))

(fn `UseObject`
  (params (InteractingCharacter :type "/Game/PNCTookit/Blueprints/Characters/BP_PNCCharacter_Parent Object Reference"))
  (returns (Success :type Boolean))
  (`parent.UseObject` InteractingCharacter)
  (if (`self.bIsUsed`)
    (set `self.bIsUsed` false)
    (`self.Clicavel`)
    (else
      (set `self.bIsUsed` true)))
  (return false))

(fn `UserConstructionScript`
  (`parent.UserConstructionScript`))