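; Trigger actor that plays a non-spatial sound while something overlaps its Box component.
; On BeginPlay it creates a 2D audio component from its Sound and Volume variables and keeps it in SoundRefer.
; Any begin overlap plays that component from the start, and any end overlap fades it out over FadeOutDuration, with no check on which actor overlaps.
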(event `self.ReceiveBeginPlay`
  (bind _returnvalue (`GameplayStatics.CreateSound2D` (`self.Sound`) (`self.Volume`) 1.0 0.0 null))
  (set `self.SoundRefer` _returnvalue))

(event `self.Box.OnComponentBeginOverlap`
  (params (OverlappedComponent :type "PrimitiveComponent Object Reference") (OtherActor :type "Actor Object Reference") (OtherComp :type "PrimitiveComponent Object Reference") (OtherBodyIndex :type Integer) (bFromSweep :type Boolean) (SweepResult :type "HitResult Structure (by ref)"))
  (`AudioComponent.Play` (`self.SoundRefer`) 0.0))

(event `self.Box.OnComponentEndOverlap`
  (params (OverlappedComponent :type "PrimitiveComponent Object Reference") (OtherActor :type "Actor Object Reference") (OtherComp :type "PrimitiveComponent Object Reference") (OtherBodyIndex :type Integer))
  (`AudioComponent.FadeOut` (`self.SoundRefer`) (`self.Fade Out Duration`) 0.0 "Linear"))

(fn `UserConstructionScript`)