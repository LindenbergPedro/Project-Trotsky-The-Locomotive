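; BP_Gaveta is an interactable locomotive drawer that slides open and closed when a character uses it.
; UseObject runs the parent's check, then toggles IsUsed and calls OpenDrawer or CloseDrawer.
; A single timeline lerps the drawer mesh's relative location, playing from start to open and reversing from end to close.
; BeginPlay creates a look-and-pick widget and caches references to it and the player character.
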(event `self.ReceiveBeginPlay`
  (`parent.ReceiveBeginPlay`)
  (bind _returnvalue (`|CreateWidget` "/Game/Blueprint/Widgets/WBP_LookAndPick.WBP_LookAndPick_C" (`GameplayStatics.GetPlayerController` 0)))
  (set `self.WBP_LookRefer` _returnvalue)
  (bind _returnvalue_2 (`GameplayStatics.GetActorOfClass` "/Game/PNCTookit/Blueprints/Characters/3D/BP_PNCCharacter_3D_Player.BP_PNCCharacter_3D_Player_C"))
  (set `self.CharacterRefer` _returnvalue_2))

(event `OpenDrawer`
  (bind (_direction _alpha) (`Timeline|Timeline_0` :!via `PlayFromStart` :!label _label)
    (:`Update`
      (`SceneComponent.K2_SetRelativeLocation` (`self.CBN_locomotive_drawer`) (`KismetMathLibrary.VLerp` (-43.0 -5.0 65.0) (-43.0 30.0 65.0) _alpha) false false))))

(event `CloseDrawer`
  (goto _label :!via `ReverseFromEnd`))

(fn `UseObject`
  (params (InteractingCharacter :type "/Game/PNCTookit/Blueprints/Characters/BP_PNCCharacter_Parent Object Reference"))
  (returns (Success :type Boolean))
  (bind _success (`parent.UseObject` InteractingCharacter))
  (if _success
    (if (`self.bIsUsed`)
      (set `self.bIsUsed` false)
      (`self.CloseDrawer`)
      (else
        (set `self.bIsUsed` true)
        (`self.OpenDrawer`))))
  (return _success))

(fn `UserConstructionScript`
  (`parent.UserConstructionScript`))