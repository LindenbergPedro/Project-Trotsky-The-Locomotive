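; BP_Drink is a drink pickup actor with a type selected by TypesDrinks (Caipiroska or Caipirinha).
; Its Pickup function sets HasDrink for a Caipiroska, while the Caipirinha case has no effect of its own.
; It then hides the static mesh, disables collision on the mesh and sphere instead of destroying the actor, and returns true.
; BeginPlay and construction only call the parent.
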(event `self.ReceiveBeginPlay`
  (`parent.ReceiveBeginPlay`))

(fn `Pickup`
  (params (Instigator :type "Actor Object Reference"))
  (returns (Success :type Boolean))
  (switch `/Game/Blueprint/Drinks/Enum_TypesDrinks` (`self.TypesDrinks`)
    (:`NewEnumerator0`
      (set `self.HasDrink` true))
    (:`NewEnumerator1`
      _))
  (`SceneComponent.SetVisibility` (`self.StaticMesh`) false false)
  (`PrimitiveComponent.SetCollisionEnabled` (`self.Sphere`) "NoCollision")
  (`PrimitiveComponent.SetCollisionEnabled` (`self.StaticMesh`) "NoCollision")
  (return true))

(fn `UserConstructionScript`
  (`parent.UserConstructionScript`))