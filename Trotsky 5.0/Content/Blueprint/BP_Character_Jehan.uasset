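; Player character Blueprint for Jehan that handles the pause input and a camera transition helper.
; Pressing B pauses the game and adds a new UIPause widget to the viewport.
; TransitionTOobjectTrue toggles the target's collision off and on, then eases the player's view to it; its false counterpart is empty.
; Click-to-move, inventory interaction and NPC dialogue logic remain as disconnected nodes that never run.
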(event `self.ReceiveBeginPlay`)

(event `MoveToLocation`
  (params (Location :type "Vector Structure")))

(event `Key|LeftMouseButton`
  (params (Key :type "Key Structure")))

(event `Key|B`
  (params (Key :type "Key Structure"))
  (:`Pressed`
    (`GameplayStatics.SetGamePaused` true)
    (bind _returnvalue (`|CreateWidget` "/Game/Interface/UI-Pause.UI-Pause_C"))
    (`UserWidget.AddToViewport` _returnvalue 0)))

(fn `TransitionTOobjectfalse`
  (params (NewParam :type "Actor Object Reference")))

(fn `TransitionTOobjectTrue`
  (params (NewParam :type "Actor Object Reference"))
  (`self.SetActorEnableCollision` NewParam false)
  (`self.SetActorEnableCollision` NewParam true)
  (`PlayerController.SetViewTargetWithBlend` (`GameplayStatics.GetPlayerController` 0) NewParam 2.0 "VTBlend_EaseInOut" 2.0 false))

(fn `UserConstructionScript`)